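; BP_ItemParent is a base item that the player picks up or inspects through interaction.
; Interactwith stores the player, then calls StartInspect if their CurrentItem is valid, otherwise PickUpItem.
; Pickup attaches the item to the player's ItemGrip, disables mesh physics and collision, and registers it as CurrentItem.
; StartInspect and Lookat are empty stubs.
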(event `/Game/ThirdPerson/Blueprints/BP_InteractInterface.LookAt`
  (params (PlayerChar :type "/Game/ThirdPerson/Blueprints/BP_ThirdPersonCharacter Object Reference")))

(event `/Game/ThirdPerson/Blueprints/BP_InteractInterface.InteractWith`
  (params (PlayerChar :type "/Game/ThirdPerson/Blueprints/BP_ThirdPersonCharacter Object Reference"))
  (bind _output_get (set `self.Player` PlayerChar))
  (`/Game/ThirdPerson/Blueprints/BP_ThirdPersonCharacter.CurrentItem` _output_get
    (:`then`
      (`self.StartInspect`))
    (:`else`
      (`self.PickUpItem`))))

(fn `PickUpItem`
  (bind _staticmesh (`self.StaticMesh`))
  (`self.K2_AttachToComponent` (`/Game/ThirdPerson/Blueprints/BP_ThirdPersonCharacter.ItemGrip` (`self.Player`)) "None" "SnapToTarget" "SnapToTarget" "KeepRelative")
  (`PrimitiveComponent.SetSimulatePhysics` _staticmesh false)
  (`PrimitiveComponent.SetCollisionEnabled` _staticmesh "NoCollision")
  (set `/Game/ThirdPerson/Blueprints/BP_ThirdPersonCharacter.CurrentItem` self (`self.Player`)))

(fn `StartInspect`)

(fn `UserConstructionScript`)
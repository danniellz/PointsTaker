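; BP_Chaser is an AI enemy character that wanders, chases sighted pawns and penalizes the player on contact.
; It patrols by looping AIMoveTo to random reachable nearby points from BeginPlay.
; PawnSensing triggers a faster chase of the seen pawn, returning to slower patrol when the move succeeds.
; Capsule hits launch BP_ThirdPersonCharacter along a fixed vector, deducting BP_PlayerState score or applying damage once none remains.
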(event `AiPatrol`
  ;[1 1 1] AI patrol
  (`|AIMoveTo` self (`NavigationSystemV1.K2_GetRandomReachablePointInRadius` (`self.K2_GetActorLocation`) 1000.0 null null) null :!label _label
    (:`OnSuccess`
      (`KismetSystemLibrary.Delay` 1.0)
      (goto _label))))

(event `self.ReceiveBeginPlay`
  ;[1 1 1] AI
  (`self.AiPatrol`))

(event `self.PawnSensing.OnSeePawn`
  (params (Pawn :type "Pawn Object Reference"))
  ;[1 1 1] On See
  (set `self.isSeeing` true)
  (`self.FollowPlayer`))

(event `FollowPlayer`
  (bind _charactermovement (`self.CharacterMovement`))
  ;[1 1 1] On See
  (if (`self.isSeeing`)
    (set `CharacterMovementComponent.MaxWalkSpeed` 700.0 _charactermovement)
    (`|AIMoveTo` self (0.0 0.0 0.0) (stale `self.PawnSensing.OnSeePawn` Pawn)
      (:`OnSuccess`
        (set `CharacterMovementComponent.MaxWalkSpeed` 300.0 (`self.CharacterMovement`))))
    (else
      (set `CharacterMovementComponent.MaxWalkSpeed` 300.0 _charactermovement)
      (set `self.isSeeing` false)))
  (`self.AiPatrol`))

(event `self.CapsuleComponent.OnComponentHit`
  (params (HitComponent :type "PrimitiveComponent Object Reference") (OtherActor :type "Actor Object Reference") (OtherComp :type "PrimitiveComponent Object Reference") (NormalImpulse :type "Vector Structure") (Hit :type "HitResult Structure (by ref)"))
  ;[1 1 1] Hit event
  (bind _asbp_third_person_character (cast `/Game/ThirdPerson/Blueprints/BP_ThirdPersonCharacter` OtherActor))
  ;;[1 1 1] Subtract Points and if points = 0, apply damage
  (bind _asbp_player_state (cast `/Game/ThirdPerson/Blueprints/BP_PlayerState` (`Pawn.PlayerState` _asbp_third_person_character)))
  (`self.LaunchCharacter` _asbp_third_person_character (800.0 800.0 300.0) false false)
  (bind _player_score (`/Game/ThirdPerson/Blueprints/BP_PlayerState.player_score` _asbp_player_state))
  (if (<= _player_score 0)
    (set `/Game/ThirdPerson/Blueprints/BP_PlayerState.player_score` 0 _asbp_player_state)
    (`GameplayStatics.ApplyDamage` _asbp_third_person_character 10.0)
    (else
      (set `/Game/ThirdPerson/Blueprints/BP_PlayerState.player_score` (- _player_score 5) _asbp_player_state))))

(fn `UserConstructionScript`)
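; BP_Chaser is an enemy AI character that wanders randomly and chases the player on sight.
; PawnSensing triggers a faster AIMoveTo pursuit, and a retriggerable delay restores patrol after sightings stop; dead players also trigger patrol.
; Capsule hits launch the player with a kick sound and deduct score, spawning temporary BP_PointLost feedback.
; Once score is depleted, hits apply damage instead, throttled by a resetting DoOnce.
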(event `AiPatrol`
  ;[1 1 1] AI patrol
  (set `CharacterMovementComponent.MaxWalkSpeed` 300.0 (`self.CharacterMovement`))
  (`|AIMoveTo` self (`NavigationSystemV1.K2_GetRandomReachablePointInRadius` (`self.K2_GetActorLocation`) 1000.0 null null) null :!label _label
    (:`OnSuccess`
      (`KismetSystemLibrary.Delay` 1.0)
      (goto _label))))

(event `self.ReceiveBeginPlay`
  ;[1 1 1] AI
  (`self.AiPatrol`))

(event `self.PawnSensing.OnSeePawn`
  (params (Pawn :type "Pawn Object Reference"))
  ;[1 1 1] On See
  (`|ExecutionSequence`
    (:`then_0`
      (bind _asbp_third_person_character (cast `/Game/ThirdPerson/Blueprints/BP_ThirdPersonCharacter` Pawn))
      (if (`/Game/ThirdPerson/Blueprints/BP_ThirdPersonCharacter.Dead?` _asbp_third_person_character)
        (`self.AiPatrol` :!label _label_2)
        (else
          (set `CharacterMovementComponent.MaxWalkSpeed` 700.0 (`self.CharacterMovement`))
          (`|AIMoveTo` self (0.0 0.0 0.0) Pawn))))
    (:`then_1`
      (`KismetSystemLibrary.RetriggerableDelay` 5.0)
      (goto _label_2))))

(event `self.CapsuleComponent.OnComponentHit`
  (params (HitComponent :type "PrimitiveComponent Object Reference") (OtherActor :type "Actor Object Reference") (OtherComp :type "PrimitiveComponent Object Reference") (NormalImpulse :type "Vector Structure") (Hit :type "HitResult Structure (by ref)"))
  ;[1 1 1] Hit event
  (bind _asbp_third_person_character (cast `/Game/ThirdPerson/Blueprints/BP_ThirdPersonCharacter` OtherActor))
  ;;[1 1 1] Subtract Points and if points = 0, apply damage
  (`GameplayStatics.PlaySoundAtLocation` "/Game/Audio/kick.kick" (`self.K2_GetActorLocation` _asbp_third_person_character) (struct) 1.0 1.0 0.0 null null null null)
  (bind _asbp_player_state (cast `/Game/ThirdPerson/Blueprints/BP_PlayerState` (`Pawn.PlayerState` _asbp_third_person_character)))
  (`self.LaunchCharacter` _asbp_third_person_character (800.0 800.0 300.0) false false)
  (bind _player_score (`/Game/ThirdPerson/Blueprints/BP_PlayerState.player_score` _asbp_player_state))
  (if (<= _player_score 0)
    (set `/Game/ThirdPerson/Blueprints/BP_PlayerState.player_score` 0 _asbp_player_state)
    (`/Engine/EditorBlueprintResources/StandardMacros.DoOnce` false :!label _label_3
      (:`Completed`
        (`GameplayStatics.ApplyDamage` _asbp_third_person_character 10.0)
        (`KismetSystemLibrary.Delay` 0.3)
        (goto _label_3 :!via `Reset`)))
    (else
      (set `/Game/ThirdPerson/Blueprints/BP_PlayerState.player_score` (- _player_score 5) _asbp_player_state)
      (bind (_returnvalue_location _returnvalue_rotation _returnvalue_scale) (`KismetMathLibrary.BreakTransform` (`self.GetTransform` _asbp_third_person_character)))
      (`|SpawnActorFromClass` "/Game/ThirdPerson/Blueprints/BP_PointLost.BP_PointLost_C" (`KismetMathLibrary.MakeTransform` (+ _returnvalue_location (0.0 0.0 100.0)) _returnvalue_rotation _returnvalue_scale) "Undefined" "OverrideRootScale" null null)
      (`GameplayStatics.PlaySound2D` "/Game/Audio/point.point" 1.0 2.0 0.0 null null)
      (`KismetSystemLibrary.Delay` 3.0)
      (bind _outactors (`GameplayStatics.GetAllActorsOfClass` "/Game/ThirdPerson/Blueprints/BP_PointLost.BP_PointLost_C"))
      (`self.K2_DestroyActor` _outactors))))

(fn `UserConstructionScript`)